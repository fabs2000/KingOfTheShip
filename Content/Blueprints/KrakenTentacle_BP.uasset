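; Kraken tentacle actor that rises to a boat position, bobs, slams and retreats, then destroys itself about seven seconds after it starts ticking.
; BeginPlay runs a chain of eased latent MoveComponentTo steps on MPBody through offsets from the actor's location, ending at EndPosition.
; The quicker final bob triggers LaunchObjects, force feedback on all player controllers and two slam sounds.
; Tick plays MPBody's animation and handles the delayed destroy.
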(event `self.ReceiveBeginPlay`
  (`self.KrakenMovement`))

(event `self.ReceiveTick`
  (params (DeltaSeconds :type "Float (single-precision)"))
  (`SkeletalMeshComponent.Play` (`self.m_pBody`) false)
  (`KismetSystemLibrary.Delay` 7.0)
  (`self.K2_DestroyActor`))

(event `KrakenMovement`
  (bind _m_pbody (`self.m_pBody`))
  (bind _m_pbody_2 (`self.m_pBody`))
  (`KismetSystemLibrary.MoveComponentTo` _m_pbody (+ (`self.K2_GetActorLocation`) (`self.StartPosition`)) (struct :`Yaw` 90.0) true true 0.0)
  (`KismetSystemLibrary.MoveComponentTo` _m_pbody (+ (`self.K2_GetActorLocation`) (`self.BoatPosition`)) (struct :`Yaw` 90.0) true true 1.0)
  (`KismetSystemLibrary.MoveComponentTo` _m_pbody (+ (`self.K2_GetActorLocation`) (`self.BobbingStart`)) (struct :`Yaw` 90.0) true true 1.0)
  (`KismetSystemLibrary.MoveComponentTo` _m_pbody (+ (`self.K2_GetActorLocation`) (`self.BobbingEnd`)) (struct :`Yaw` 90.0) true true 1.0)
  (`KismetSystemLibrary.MoveComponentTo` _m_pbody (+ (`self.K2_GetActorLocation`) (`self.BobbingStart`)) (struct :`Yaw` 90.0) true true 1.0)
  (`KismetSystemLibrary.MoveComponentTo` _m_pbody (+ (`self.K2_GetActorLocation`) (`self.BobbingEnd`)) (struct :`Yaw` 90.0) true true 0.4)
  (`self.LaunchObjects`)
  (bind _outactors (`GameplayStatics.GetAllActorsOfClass` "/Script/Engine.PlayerController"))
  (for _array_element _outactors
    (`PlayerController.PlayDynamicForceFeedback` _array_element 1.0 0.6 true true true true))
  (`GameplayStatics.SpawnSoundAttached` "/Game/Sound/KrakenSlam_SFX.KrakenSlam_SFX" _m_pbody_2 "None" (0.0 0.0 0.0) (struct) "KeepRelativeOffset" false 1.0 1.0 0.0 null null)
  (`GameplayStatics.SpawnSoundAttached` "/Game/Sound/KrakenSlam_SFX_2.KrakenSlam_SFX_2" _m_pbody_2 "None" (0.0 0.0 0.0) (struct) "KeepRelativeOffset" false 1.0 1.0 0.0 null null)
  (`KismetSystemLibrary.Delay` 0.6)
  (`KismetSystemLibrary.MoveComponentTo` _m_pbody (+ (`self.K2_GetActorLocation`) (`self.EndPosition`)) (struct :`Yaw` 90.0) true true 1.0))

(fn `UserConstructionScript`)