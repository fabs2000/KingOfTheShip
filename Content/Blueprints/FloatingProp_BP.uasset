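; FloatingProp_BP is a prop whose static mesh bobs and tilts in an endless floating motion.
; On BeginPlay it snaps the mesh to the actor location at the minimum rotation, then starts FloatingMotion.
; That event chains two eased MoveComponentTo moves between up and down offsets and rotation limits, then calls itself again.
; Each move re-reads the actor's world location and passes it as a relative target.
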(event `self.ReceiveBeginPlay`
  (`KismetSystemLibrary.MoveComponentTo` (`self.StaticMeshComponent`) (`self.K2_GetActorLocation`) (`self.RotationMin`) true true 0.0)
  (`self.FloatingMotion`))

(event `FloatingMotion`
  (bind _staticmeshcomponent (`self.StaticMeshComponent`))
  (bind _time (`self.Time`))
  (`KismetSystemLibrary.MoveComponentTo` _staticmeshcomponent (+ (`self.K2_GetActorLocation`) (`self.UpMax`)) (`self.RotationMax`) true true _time)
  (`KismetSystemLibrary.MoveComponentTo` _staticmeshcomponent (+ (`self.K2_GetActorLocation`) (`self.DownMax`)) (`self.RotationMin`) true true _time)
  (`self.FloatingMotion`))

(fn `UserConstructionScript`)