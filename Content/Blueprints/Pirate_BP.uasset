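; Pirate character Blueprint that drives animation, VFX, sound and gamepad rumble feedback.
; Tick polls water state to toggle a per-pirate-type notification effect, splash and drowning animation flag, and plays shoot montage and muzzle FX while the weapon can shoot.
; It also watches the active effect, using resettable once-gates for timed Drunk and Speed Boost FX, and a Power Shot pickup sound.
; Notify events handle dash montage, shot sounds and force feedback.
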(event `self.ReceiveTick`
  (params (DeltaSeconds :type "Float (single-precision)"))
  (bind _mesh (`self.Mesh`))
  (bind _mesh_2 (`self.Mesh`))
  (bind _mesh_3 (`self.Mesh`))
  (`|ExecutionSequence`
    (:`then_0`
      (if (`self.m_IsInWater`)
        (`|DoOnceMultiInput` :!label _label
          (:`A Out`
            (switch `PirateType` (`self.m_PirateType`)
              (:`Captn`
                (bind _returnvalue (`NiagaraFunctionLibrary.SpawnSystemAttached` "/Game/RFX/FX_Notifications/CaptnNotifcation_FX_NS.CaptnNotifcation_FX_NS" _mesh "None" (0.0 0.0 600.0) (struct) "SnapToTargetIncludingScale")))
              (:`Parry`
                (bind _returnvalue_2 (`NiagaraFunctionLibrary.SpawnSystemAttached` "/Game/RFX/FX_Notifications/ParryNotifcation_FX_NS.ParryNotifcation_FX_NS" _mesh "None" (0.0 0.0 600.0) (struct) "SnapToTargetIncludingScale")))
              (:`Sharky`
                (bind _returnvalue_3 (`NiagaraFunctionLibrary.SpawnSystemAttached` "/Game/RFX/FX_Notifications/SharkyNotifcation_FX_NS.SharkyNotifcation_FX_NS" _mesh "None" (0.0 0.0 600.0) (struct) "SnapToTargetIncludingScale")))
              (:`Shrimp`
                (bind _returnvalue_4 (`NiagaraFunctionLibrary.SpawnSystemAttached` "/Game/RFX/FX_Notifications/ShrimpNotifcation_FX_NS.ShrimpNotifcation_FX_NS" _mesh "None" (0.0 0.0 600.0) (struct) "SnapToTargetIncludingScale")))))
          (:`Reset Out`
            (`/Engine/EditorBlueprintResources/StandardMacros.IsValid` _returnvalue
              (:`Is Valid`
                (`ActorComponent.K2_DestroyComponent` _returnvalue))
              (:`Is Not Valid`
                (`/Engine/EditorBlueprintResources/StandardMacros.IsValid` _returnvalue_2
                  (:`Is Valid`
                    (`ActorComponent.K2_DestroyComponent` _returnvalue_2))
                  (:`Is Not Valid`
                    (`/Engine/EditorBlueprintResources/StandardMacros.IsValid` _returnvalue_3
                      (:`Is Valid`
                        (`ActorComponent.K2_DestroyComponent` _returnvalue_3))
                      (:`Is Not Valid`
                        (`/Engine/EditorBlueprintResources/StandardMacros.IsValid` _returnvalue_4
                          (:`Is Valid`
                            (`ActorComponent.K2_DestroyComponent` _returnvalue_4)))))))))))
        (else
          (goto _label :!via `Reset In`))))
    (:`then_1`
      (bind _ascharacter_abp (cast `/Game/Animations/Characters/Character_ABP` (`SkeletalMeshComponent.GetAnimInstance` (`self.Mesh`))))
      (bind _output_get (set `/Game/Animations/Characters/Character_ABP.isDrowning` (`self.m_IsInWater`) _ascharacter_abp))
      (if _output_get
        (`/Engine/EditorBlueprintResources/StandardMacros.DoOnce` false :!label _label_2
          (:`Completed`
            (`NiagaraFunctionLibrary.SpawnSystemAttached` "/Game/RFX/FX_WaterSplash/WaterSplash_FX_NS.WaterSplash_FX_NS" (`self.Mesh`) "None" (0.0 0.0 0.0) (struct) "SnapToTargetIncludingScale")))
        (else
          (goto _label_2 :!via `Reset`))))
    (:`then_2`
      (bind _returnvalue_5 (`Weapon.CanShoot` (`self.Weapon`)))
      (if _returnvalue_5
        (`self.PlayAnimMontage` "/Game/Animations/Characters/Character_Anim_Montage.Character_Anim_Montage" 1.0 "AnimShoot")
        (`NiagaraFunctionLibrary.SpawnSystemAttached` "/Game/RFX/FX_PrimaryFire/PrimaryFire_FX_NS.PrimaryFire_FX_NS" (`self.ShotDirect`) "None" (0.0 0.0 0.0) (struct) "SnapToTargetIncludingScale" true)))
    (:`then_3`
      (switch `Effect` (`self.m_Effect`)
        (:`Drunk`
          (`/Engine/EditorBlueprintResources/StandardMacros.DoOnce` false :!label _label_3
            (:`Completed`
              (`GameplayStatics.SpawnSoundAttached` "/Game/Sound/Rum_PickUp_SFX.Rum_PickUp_SFX" _mesh_3 "None" (0.0 0.0 0.0) (struct) "KeepRelativeOffset" false 1.0 1.0 0.0 null null)
              (bind _returnvalue_6 (`NiagaraFunctionLibrary.SpawnSystemAttached` "/Game/RFX/FX_Drunk/Drunk_FX_NS.Drunk_FX_NS" _mesh_2 "None" (0.0 0.0 0.0) (struct) "SnapToTargetIncludingScale"))
              (set `self.m_pActiveEffect` _returnvalue_6)
              (`KismetSystemLibrary.Delay` (`self.m_EffectDuration`))
              (`ActorComponent.K2_DestroyComponent` _returnvalue_6)
              (goto _label_3 :!via `Reset`))))
        (:`SpeedBoost`
          (`/Engine/EditorBlueprintResources/StandardMacros.DoOnce` false :!label _label_4
            (:`Completed`
              (`GameplayStatics.SpawnSoundAttached` "/Game/Sound/Speed_PickUp_SFX.Speed_PickUp_SFX" _mesh_3 "None" (0.0 0.0 0.0) (struct) "KeepRelativeOffset" false 1.0 1.0 0.0 null null)
              (bind _returnvalue_7 (`NiagaraFunctionLibrary.SpawnSystemAttached` "/Game/RFX/FX_Speed/Speed_FX_NS.Speed_FX_NS" _mesh_2 "None" (0.0 0.0 0.0) (struct) "SnapToTargetIncludingScale"))
              (set `self.m_pActiveEffect` _returnvalue_7)
              (`KismetSystemLibrary.Delay` (`self.m_EffectDuration`))
              (`ActorComponent.K2_DestroyComponent` _returnvalue_7)
              (goto _label_4 :!via `Reset`))))
        (:`PowerShot`
          (`/Engine/EditorBlueprintResources/StandardMacros.DoOnce` false
            (:`Completed`
              (`GameplayStatics.SpawnSoundAttached` "/Game/Sound/PowerShot_PickUp_SFX.PowerShot_PickUp_SFX" _mesh_3 "None" (0.0 0.0 0.0) (struct) "KeepRelativeOffset" false 1.0 1.0 0.0 null null))))))))

(event `self.NotifyDash`
  (`self.PlayAnimMontage` "/Game/Animations/Characters/Character_Anim_Montage.Character_Anim_Montage" 1.0 "AnimDash"))

(event `self.NotifyShoot`
  (`GameplayStatics.SpawnSoundAttached` "/Game/Sound/Shot_SFX_V2.Shot_SFX_V2" (`self.Mesh`) "None" (0.0 0.0 0.0) (struct) "KeepRelativeOffset" false 1.0 1.0 0.0 null null)
  (bind _asplayer_controller (cast `PlayerController` (`self.GetController`)))
  (`PlayerController.PlayDynamicForceFeedback` _asplayer_controller 0.5 0.4 false true false true))

(event `self.NotifyPowerShot`
  (`GameplayStatics.SpawnSoundAttached` "/Game/Sound/PowerShot_SFX.PowerShot_SFX" (`self.Mesh`) "None" (0.0 0.0 0.0) (struct) "KeepRelativeOffset" false 1.0 1.0 0.0 null null)
  (bind _asplayer_controller (cast `PlayerController` (`self.GetController`)))
  (`PlayerController.PlayDynamicForceFeedback` _asplayer_controller 1.0 0.4 true false true false))

(event `self.NotifyRecover`
  (bind _asplayer_controller (cast `PlayerController` (`self.GetController`)))
  (`PlayerController.PlayDynamicForceFeedback` _asplayer_controller 0.4 0.2 false true false true))

(fn `UserConstructionScript`)