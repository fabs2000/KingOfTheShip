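; CharInd_BP is a pawn Blueprint that gives controller rumble feedback for active and directional notifications.
; NotifyActive, NotifyGoLeft and NotifyGoRight each cast the pawn's controller to PlayerController and play dynamic force feedback.
; Active pulses both small motors at full strength, while left and right give a weaker, shorter pulse on the matching side's small motor, so direction is felt by hand.
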(event `self.ReceiveBeginPlay`)

(event `self.NotifyActive`
  (bind _asplayer_controller (cast `PlayerController` (`self.GetController`)))
  (`PlayerController.PlayDynamicForceFeedback` _asplayer_controller 1.0 0.4 false true false true))

(event `self.NotifyGoLeft`
  (bind _asplayer_controller (cast `PlayerController` (`self.GetController`)))
  (`PlayerController.PlayDynamicForceFeedback` _asplayer_controller 0.3 0.2 false true false false))

(event `self.NotifyGoRight`
  (bind _asplayer_controller (cast `PlayerController` (`self.GetController`)))
  (`PlayerController.PlayDynamicForceFeedback` _asplayer_controller 0.3 0.2 false false false true))

(fn `UserConstructionScript`)