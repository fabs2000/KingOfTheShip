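; Kraken actor that provides audio and warning effects for the Kraken event.
; PlayKrakenSounds checks the game mode's MKrakenEvent flag, fades in an attached looping sound, then after a fixed delay fades it out only if the event has ended.
; SpawnIndicator shows a Niagara notification above a given spawn point and destroys it shortly afterwards.
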(event `self.PlayKrakenSounds`
  (bind _asgame_mode_bp (cast `/Game/Blueprints/GameMode_BP` (`GameplayStatics.GetGameMode`)))
  (bind _m_krakenevent (`KingOfTheShip_MainGameModeBase.m_KrakenEvent` _asgame_mode_bp))
  (if _m_krakenevent
    (bind _returnvalue (`GameplayStatics.SpawnSoundAttached` "/Game/Sound/KrakenLoop_SFX.KrakenLoop_SFX" (`self.DefaultSceneRoot`) "None" (0.0 0.0 0.0) (struct) "KeepRelativeOffset" false 1.0 1.0 0.0 null null))
    (`AudioComponent.FadeIn` _returnvalue 2.5 0.7 0.0)
    (`KismetSystemLibrary.Delay` 39.0)
    (if (not _m_krakenevent)
      (`AudioComponent.FadeOut` _returnvalue 2.5 0.1))))

(event `self.SpawnIndicator`
  (params (spawnPoint :type "TargetPoint Object Reference"))
  (bind _returnvalue (`NiagaraFunctionLibrary.SpawnSystemAtLocation` "/Game/RFX/FX_Notifications/KrakenNotification_FX_NS.KrakenNotification_FX_NS" (+ (`SceneComponent.K2_GetComponentLocation` (`Actor.RootComponent` spawnPoint)) (0.0 0.0 300.0)) (struct) false))
  (`KismetSystemLibrary.Delay` 2.0)
  (`/Engine/EditorBlueprintResources/StandardMacros.IsValid` _returnvalue
    (:`Is Valid`
      (`ActorComponent.K2_DestroyComponent` _returnvalue))))

(fn `UserConstructionScript`)